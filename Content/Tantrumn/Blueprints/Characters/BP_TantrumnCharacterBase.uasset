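; BP_TantrumnCharacterBase is the base character Blueprint for Tantrumn, turning Enhanced Input actions into movement, jumping and look control.
; Separate forward and right actions feed CharacterMovement input vectors along the controller actor's axes, so movement follows controller orientation.
; Look actions drive controller yaw and inverted pitch, while the jump action calls Jump whenever triggered.
; BeginPlay, overlap, Tick and the construction script are empty.
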(event `EnhancedInput|/Game/Tantrumn/InputActions/IA_Jump`
  (params (ActionValue :type Boolean) (ElapsedSeconds :type "Float (double-precision)") (TriggeredSeconds :type "Float (double-precision)") (InputAction :type "InputAction Object Reference" :default "/Game/Tantrumn/InputActions/IA_Jump.IA_Jump"))
  (:`Triggered`
    (`self.Jump`)))

(event `EnhancedInput|/Game/Tantrumn/InputActions/IA_MoveForward`
  (params (ActionValue :type "Float (double-precision)") (ElapsedSeconds :type "Float (double-precision)") (TriggeredSeconds :type "Float (double-precision)") (InputAction :type "InputAction Object Reference" :default "/Game/Tantrumn/InputActions/IA_MoveForward.IA_MoveForward"))
  (:`Triggered`
    (`PawnMovementComponent.AddInputVector` (`self.CharacterMovement`) (* (`self.GetActorForwardVector` (`self.GetController`)) ActionValue) false)))

(event `EnhancedInput|/Game/Tantrumn/InputActions/IA_MoveRight`
  (params (ActionValue :type "Float (double-precision)") (ElapsedSeconds :type "Float (double-precision)") (TriggeredSeconds :type "Float (double-precision)") (InputAction :type "InputAction Object Reference" :default "/Game/Tantrumn/InputActions/IA_MoveRight.IA_MoveRight"))
  (:`Triggered`
    (`PawnMovementComponent.AddInputVector` (`self.CharacterMovement`) (* (`self.GetActorRightVector` (`self.GetController`)) ActionValue) false)))

(event `EnhancedInput|/Game/Tantrumn/InputActions/IA_LookUp`
  (params (ActionValue :type "Float (double-precision)") (ElapsedSeconds :type "Float (double-precision)") (TriggeredSeconds :type "Float (double-precision)") (InputAction :type "InputAction Object Reference" :default "/Game/Tantrumn/InputActions/IA_LookUp.IA_LookUp"))
  (:`Triggered`
    (`self.AddControllerPitchInput` (* ActionValue -1.0))))

(event `EnhancedInput|/Game/Tantrumn/InputActions/IA_LookRight`
  (params (ActionValue :type "Float (double-precision)") (ElapsedSeconds :type "Float (double-precision)") (TriggeredSeconds :type "Float (double-precision)") (InputAction :type "InputAction Object Reference" :default "/Game/Tantrumn/InputActions/IA_LookRight.IA_LookRight"))
  (:`Triggered`
    (`self.AddControllerYawInput` (* ActionValue 1.0))))

(fn `UserConstructionScript`)