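; BP_Character is a character Blueprint that measures and prints jump metrics, apparently for tuning movement.
; OnJumped stores the start time and position, and OnLanded prints total air time and straight-line distance from that start point.
; Tick compares current vertical velocity with the previous frame's to detect the apex as a positive-to-negative flip, then prints the time taken to reach it.
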(event `self.OnJumped`
  ;[1 1 1] Jump Time
  (set `self.JumpStartTime` (`GameplayStatics.GetTimeSeconds`))
  (set `self.JumpStartPosition` (`self.K2_GetActorLocation`)))

(event `self.OnLanded`
  (params (Hit :type "HitResult Structure (by ref)"))
  ;[1 1 1] Jump Time
  (`KismetSystemLibrary.PrintString` (`KismetStringLibrary.Concat_StrStr` "Fly Time: " (`KismetStringLibrary.Conv_DoubleToString` (- (`GameplayStatics.GetTimeSeconds`) (`self.JumpStartTime`)))))
  (`KismetSystemLibrary.PrintString` (`KismetStringLibrary.Concat_StrStr` "Land Distance: " (`KismetStringLibrary.Conv_DoubleToString` (`KismetMathLibrary.Vector_Distance` (`self.K2_GetActorLocation`) (`self.JumpStartPosition`))))))

(event `self.ReceiveTick`
  (params (DeltaSeconds :type "Float (single-precision)"))
  (bind (_returnvalue_x _returnvalue_y _returnvalue_z) (`KismetMathLibrary.BreakVector` (`self.GetVelocity`)))
  (bind (_lastvelocity_x _lastvelocity_y _lastvelocity_z) (`KismetMathLibrary.BreakVector` (`self.LastVelocity`)))
  ;[1 1 1] Apex Jump Timer
  (if (and (< _returnvalue_z 0.0) (> _lastvelocity_z 0.0))
    (`KismetSystemLibrary.PrintString` (`KismetStringLibrary.Concat_StrStr` "Apex Time: " (`KismetStringLibrary.Conv_DoubleToString` (- (`GameplayStatics.GetTimeSeconds`) (`self.JumpStartTime`))))))
  (set `self.LastVelocity` (`self.GetVelocity`)))

(fn `UserConstructionScript`
  (`parent.UserConstructionScript`))